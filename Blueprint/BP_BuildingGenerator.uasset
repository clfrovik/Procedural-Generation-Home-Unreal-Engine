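; Procedural building generator that assembles a box-shaped building from modular meshes in the construction script.
; Width, Depth and Height loops place rotated window-mesh instances on four sides, spaced by that mesh's local bounds.
; Optional roof and floor grids both add to the roof instanced mesh; the floor mesh supplies only the floor grid's spacing and Z offset.
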(fn `UserConstructionScript`
  (bind (_min _max) (`StaticMeshComponent.GetLocalBounds` (`self.Instanced Window Mesh`)))
  (bind (_min_2 _max_2) (`StaticMeshComponent.GetLocalBounds` (`self.Instanced Window Mesh`)))
  (bind (_min_3 _max_3) (`StaticMeshComponent.GetLocalBounds` (`self.Instanced Window Mesh`)))
  (bind (_min_4 _max_4) (`StaticMeshComponent.GetLocalBounds` (`self.Instanced Window Mesh`)))
  (bind (_min_5 _max_5) (`StaticMeshComponent.GetLocalBounds` (`self.Instanced Floor Mesh`)))
  (bind (_min_6 _max_6) (`StaticMeshComponent.GetLocalBounds` (`self.Instanced Window Mesh`)))
  (`StaticMeshComponent.SetStaticMesh` (`self.Instanced Window Mesh`) (`self.Select Window Mesh`))
  (`StaticMeshComponent.SetStaticMesh` (`self.Instanced Roof Mesh`) (`self.Select Roof Mesh`))
  (`StaticMeshComponent.SetStaticMesh` (`self.Instanced Floor Mesh`) (`self.Select Floor Mesh`))
  (`|ExecutionSequence`
    (:`then_0`
      ;[1 1 1] Front
      (for _index (range (`self.Width`))
        (for _index_2 (range (`self.Height`))
          (`InstancedStaticMeshComponent.AddInstance` (`self.Instanced Window Mesh`) (`KismetMathLibrary.MakeTransform` (`KismetMathLibrary.MakeVector` (* _index (.x _max_6)) 0.0 (* _index_2 (.z _max_6)))) false))))
    (:`then_1`
      ;[0.513 0.6066 1] Back
      (for _index_3 (range (`self.Width`))
        (for _index_4 (range (`self.Height`))
          (`InstancedStaticMeshComponent.AddInstance` (`self.Instanced Window Mesh`) (`KismetMathLibrary.MakeTransform` (`KismetMathLibrary.MakeVector` (+ (* _index_3 (.x _max)) (.x _max)) (* (.x _max) (`self.Depth`) -1.0) (* _index_4 (.z _max))) (struct :`Yaw` 180.0)) false))))
    (:`then_2`
      ;[1 1 1] Left
      (for _index_5 (range (`self.Depth`))
        (for _index_6 (range (`self.Height`))
          (`InstancedStaticMeshComponent.AddInstance` (`self.Instanced Window Mesh`) (`KismetMathLibrary.MakeTransform` (`KismetMathLibrary.MakeVector` 0.0 (- (* (* _index_5 (.x _max_2)) -1.0) (.x _max_2)) (* _index_6 (.z _max_2))) (struct :`Yaw` 90.0)) false))))
    (:`then_3`
      ;[1 1 1] Right
      (for _index_7 (range (`self.Depth`))
        (for _index_8 (range (`self.Height`))
          (`InstancedStaticMeshComponent.AddInstance` (`self.Instanced Window Mesh`) (`KismetMathLibrary.MakeTransform` (`KismetMathLibrary.MakeVector` (* (.x _max_3) (`self.Width`)) (* (* _index_7 (.x _max_3)) -1.0) (* _index_8 (.z _max_3))) (struct :`Yaw` -90.0)) false))))
    (:`then_4`
      ;[1 1 1] Roof
      (if (`self.RoodCreate?`)
        (for _index_9 (range (`self.Width`))
          (for _index_10 (range (`self.Depth`))
            (`InstancedStaticMeshComponent.AddInstance` (`self.Instanced Roof Mesh`) (`KismetMathLibrary.MakeTransform` (`KismetMathLibrary.MakeVector` (* _index_9 (.x _max_4)) (- (* _index_10 (.x _max_4) -1.0) (.x _max_4)) (* (`self.Height`) (.z _max_4))) (struct :`Yaw` 90.0)) false)))))
    (:`then_5`
      ;[1 1 1] Floor
      (if (`self.FloorCreate?`)
        (for _index_11 (range (`self.Width`))
          (for _index_12 (range (`self.Depth`))
            (`InstancedStaticMeshComponent.AddInstance` (`self.Instanced Roof Mesh`) (`KismetMathLibrary.MakeTransform` (`KismetMathLibrary.MakeVector` (* _index_11 (.x _max_5)) (- (* _index_12 (.x _max_5) -1.0) (.x _max_5)) (* (`self.Height`) (.z _min_5))) (struct :`Yaw` 90.0)) false)))))))