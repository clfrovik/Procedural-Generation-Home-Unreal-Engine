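; BP_BuildingCollector is an actor that stacks BP_BuildingGenerator actors vertically to assemble a building.
; Each AddFloor event spawns a generator at the Scene component's relative X and Y, at height MaxZ, then attaches it to itself with KeepRelative rules.
; MaxZ then grows by the generator's Height times its window mesh's upper Z bound.
; The construction script resets MaxZ to zero.
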(event `Add Floor`
  (bind _returnvalue (`SceneComponent.GetRelativeTransform` (`self.Scene`)))
  (bind _returnvalue_2 (`|SpawnActorFromClass` "/Game/ProcBuilding/Blueprint/BP_BuildingGenerator.BP_BuildingGenerator_C" (`KismetMathLibrary.MakeTransform` (`KismetMathLibrary.MakeVector` (.x (.location _returnvalue)) (.y (.location _returnvalue)) (`self.Max Z`))) "Undefined" "OverrideRootScale" null null))
  (set `self.Max Z` (+ (`self.Max Z`) (* (`/Game/ProcBuilding/Blueprint/BP_BuildingGenerator.Height` _returnvalue_2) (.z (`.Max` (`StaticMeshComponent.GetLocalBounds` (`/Game/ProcBuilding/Blueprint/BP_BuildingGenerator.Instanced Window Mesh` _returnvalue_2)))))))
  (`self.K2_AttachToActor` _returnvalue_2 self "None" "KeepRelative" "KeepRelative" "KeepRelative" true))

(fn `UserConstructionScript`
  (set `self.Max Z` 0.0))