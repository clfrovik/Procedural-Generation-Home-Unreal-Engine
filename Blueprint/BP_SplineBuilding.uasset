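; Spline-driven procedural building generator that assembles a multi-storey building in the construction script.
; It stacks spline meshes by section length and Height, with SetSplineMesh cycling ground, middle and top-floor mesh arrays.
; Optional pillars and wall props sit at section ends, roof props scatter randomly around the averaged spline centre, and a roof-edge mesh follows the spline.
; Optional floor and roof are procedural-mesh triangle fans from that centre to spline points.
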(fn `Get End Pos/Tangent`
  (params (Index :type Integer))
  (returns (Position :type "Vector Structure") (Tangent :type "Vector Structure"))
  (bind _spline (`self.Spline`))
  (bind _returnvalue (* (+ Index 1) (`self.SectionLenght`)))
  (return (`SplineComponent.GetLocationAtDistanceAlongSpline` _spline _returnvalue "Local") (`KismetMathLibrary.ClampVectorSize` (`SplineComponent.GetTangentAtDistanceAlongSpline` _spline _returnvalue "Local") 0.0 (`self.SectionLenght`))))

(fn `Get Section`
  (returns (Vectices :type "Array of Vector Structure") (Triangles :type "Array of Integer") (Normals :type "Array of Vector Structure") (UVs :type "Array of Vector2D Structure") (Tangents :type "Array of ProcMeshTangent Structure"))
  (bind (_vertices _triangles _normals _uvs _tangents) (`KismetProceduralMeshLibrary.GetSectionFromStaticMesh` "/Game/Megascans/NewFolder/фц5в_Плоскость.фц5в_Плоскость"))
  (set `self.Vertices_0` _vertices)
  (set `self.Triangles` _triangles)
  (set `self.Normals` _normals)
  (set `self.UVs` _uvs)
  (set `self.Tangents` _tangents)
  (return (`self.Vertices_0`) (`self.Triangles`) (`self.Normals`) (`self.UVs`) (`self.Tangents`)))

(fn `Get Start Pos/Tangent`
  (params (Index :type Integer))
  (returns (`Start Location` :type "Vector Structure") (`Start Tangent` :type "Vector Structure"))
  (bind _spline (`self.Spline`))
  (bind _returnvalue (* Index (`self.SectionLenght`)))
  (return (`SplineComponent.GetLocationAtDistanceAlongSpline` _spline _returnvalue "Local") (`KismetMathLibrary.ClampVectorSize` (`SplineComponent.GetTangentAtDistanceAlongSpline` _spline _returnvalue "Local") 0.0 (`self.SectionLenght`))))

(fn `Set Spline Mesh`
  (`|ExecutionSequence`
    (:`then_0`
      ;[0.5136 1 0.92] Set Mesh Wall
      ;;[1 1 1] Set Mesh One floor
      (if (== (`self.IndexHeightCurrent`) 0)
        (for _ (range (+ (`self.LoopIndex`) 1))
          (set `self.SplineMesh` (`|GetArrayItem` (`self.Static Mesh One Floor`) (`self.Index Mesh`)))
          (set `self.Index Mesh` (+ (`self.Index Mesh`) 1))
          (if (>= (`self.Index Mesh`) (`KismetArrayLibrary.Array_Length` (`self.Static Mesh One Floor`)))
            (set `self.Index Mesh` 0)))
        (else
          ;;[1 1 1] Set Mesh Roofs
          (if (> (`self.IndexHeightCurrent`) 0)
            (if (== (- (`self.Height`) 1) (`self.IndexHeightCurrent`))
              (for _ (range (+ (`self.LoopIndex`) 1))
                (set `self.SplineMesh` (`|GetArrayItem` (`self.Static Mesh Roof`) (`self.Index Mesh Roof`)))
                (set `self.Index Mesh Roof` (+ (`self.Index Mesh Roof`) 1))
                (if (>= (`self.Index Mesh Roof`) (`KismetArrayLibrary.Array_Length` (`self.Static Mesh Roof`)))
                  (set `self.Index Mesh Roof` 0)))
              (else
                ;;[1 1 1] Set Mesh Props Middle Floor
                (for _ (range (+ (`self.LoopIndex`) 1))
                  (set `self.SplineMesh` (`|GetArrayItem` (`self.Statc Mesh Middle Floors`) (`self.Index Middle floor mesh`)))
                  (set `self.Index Middle floor mesh` (+ (`self.Index Middle floor mesh`) 1))
                  (if (>= (`self.Index Middle floor mesh`) (`KismetArrayLibrary.Array_Length` (`self.Statc Mesh Middle Floors`)))
                    (set `self.Index Middle floor mesh` 0)))))))))
    (:`then_1`
      ;[0.5021 0.69 1] Props
      ;;[1 1 1] Props Wall
      (for _ (range (+ (`self.LoopIndex`) 1))
        (set `self.Spline Mesh Props` (`|GetArrayItem` (`self.StaticMeshPropsWall`) (`self.Index Props Wall`)))
        (set `self.Index Props Wall` (+ (`self.Index Props Wall`) 1))
        (if (>= (`self.Index Props Wall`) (`KismetArrayLibrary.Array_Length` (`self.StaticMeshPropsWall`)))
          (set `self.Index Props Wall` 0))))
    (:`then_2`
      ;;[1 1 1] Props Roof
      (for _ (range (+ (`self.LoopIndex`) 1))
        (set `self.Roof Props Mesh` (`|GetArrayItem` (`self.Roof Prop Mesh`) (`self.Index Roof Props`)))
        (set `self.Index Roof Props` (+ (`self.Index Roof Props`) 1))
        (if (>= (`self.Index Roof Props`) (`KismetArrayLibrary.Array_Length` (`self.Roof Prop Mesh`)))
          (set `self.Index Roof Props` 0))))))

(fn `UserConstructionScript`
  (bind _returnvalue_x (`KismetMathLibrary.BreakVector` (`self.GetActorScale3D`)))
  (bind _randomize_x_props (`self.Randomize X Props`))
  (bind _loopindex (`self.LoopIndex`))
  (bind _spline (`self.Spline`))
  (bind _randomize_y_props (`self.Randomize Y Props`))
  (bind _spline_2 (`self.Spline`))
  (bind _vertices (`self.Vertices`))
  (bind _height (`self.Height`))
  (bind _loopindex_2 (`self.LoopIndex`))
  (bind _loopindex_3 (`self.LoopIndex`))
  (bind _spline_3 (`self.Spline`))
  (bind _spline_4 (`self.Spline`))
  (bind _spline_5 (`self.Spline`))
  (bind _vertices_2 (`self.Vertices`))
  (bind _returnvalue (`SplineComponent.GetSplineLength` _spline_5))
  (bind _returnvalue_2 (`SplineComponent.GetTransformAtSplinePoint` _spline (`self.Index_A`) "Local" false))
  (bind _returnvalue_3 (`SplineComponent.GetSplineLength` _spline_4))
  (bind (_min _max) (`StaticMeshComponent.GetLocalBounds` (`self.SplineMeshComponent`)))
  (bind _returnvalue_4 (`SplineComponent.GetSplineLength` _spline_2))
  (bind _returnvalue_location (`KismetMathLibrary.BreakTransform` (`SplineComponent.GetTransformAtSplinePoint` _spline_3 (`self.Index B`) "Local" false)))
  (bind _returnvalue_5 (`KismetMathLibrary.FTrunc` _returnvalue))
  (bind _returnvalue_6 (`SplineComponent.GetTransformAtSplinePoint` _spline (+ (`self.Index_A`) 1) "Local" false))
  (bind _returnvalue_7 (`KismetMathLibrary.FTrunc` _returnvalue_3))
  (bind _returnvalue_8 (`KismetMathLibrary.FTrunc` _returnvalue_4))
  (bind _returnvalue_location_2 (`KismetMathLibrary.BreakTransform` (`SplineComponent.GetTransformAtSplinePoint` _spline_3 (+ (`self.Index B`) 1) "Local" false)))
  (bind _returnvalue_9 (* (`self.Height`) (.z (`.Max` (`StaticMeshComponent.GetLocalBounds` (`self.SplineMeshComponent`))))))
  (`SplineComponent.SetClosedLoop` (`self.Spline`) (`self.In Closed Loop`) true)
  (if (`self.AllowScaling?`)
    (set `self.SectionLenght` (* _returnvalue_x 100.0)))
  (`|ExecutionSequence`
    (:`then_0`
      ;[1 1 1] Roof Props
      (`|ExecutionSequence`
        (:`then_0`
          (if (`self.Create Roof Props?`)
            (for _index (range (+ _returnvalue_7 1))
              (bind _returnvalue_location_3 (`KismetMathLibrary.BreakTransform` (`SplineComponent.GetTransformAtDistanceAlongSpline` _spline_4 (* (/ (`KismetMathLibrary.Conv_IntToDouble` _index) _returnvalue_7) _returnvalue_3) "Local" false)))
              (bind _output_get (set `self.Vectors` (+ _returnvalue_location_3 (`self.Vectors`)))))
            (for _index_2 (range (`self.Height`))
              (set `self.IndexHeightCurrent` _index_2))
            (for _ (range (+ (`self.Count Props Roof`) 1))
              (bind (_returnvalue_x_2 _returnvalue_y) (`KismetMathLibrary.BreakVector` (/ _output_get _returnvalue_3)))
              (set `self.X pos` _returnvalue_x_2)
              (set `self.Y pos` _returnvalue_y)
              (bind _returnvalue_10 (`AddComponent|NODE_AddSplineMeshComponent-8` :`RelativeTransform` (`KismetMathLibrary.MakeTransform` (`KismetMathLibrary.MakeVector` 0.0 0.0 (* (`self.Height`) (.z (`.Max` (`StaticMeshComponent.GetLocalBounds` (`self.SplineMeshComponent`)))))))))
              (bind _output_get_2 (set `self.SplineMeshComponent` _returnvalue_10))
              (`self.Set Spline Mesh`)
              (`StaticMeshComponent.SetStaticMesh` _output_get_2 (`self.Roof Props Mesh`))
              (`SplineMeshComponent.SetForwardAxis` (`self.SplineMeshComponent`) "X" true)
              (`self.Get End Pos/Tangent` _loopindex)
              (`SceneComponent.K2_SetRelativeTransform` (`self.SplineMeshComponent`) (`KismetMathLibrary.MakeTransform` (`KismetMathLibrary.MakeVector` (+ (`self.X pos`) (`KismetMathLibrary.RandomIntegerInRange` (* _randomize_x_props -1) _randomize_x_props)) (+ (`self.Y pos`) (`KismetMathLibrary.RandomIntegerInRange` (* _randomize_y_props -1) _randomize_y_props)) (+ (* (`self.Height`) (.z (`StaticMeshComponent.GetLocalBounds` (`self.SplineMeshComponent`)))) (`self.Distance Roof Props`))) (`SplineComponent.GetRotationAtDistanceAlongSpline` (`self.Spline`) (* (+ _loopindex 1) (`self.SectionLenght`)) "Local")) false false))))))
    (:`then_1`
      ;[1 1 1] Pillar
      (if (`self.Create Pillar?`)
        (for _index_3 (range (+ (`KismetMathLibrary.FTrunc` (/ (`SplineComponent.GetSplineLength` (`self.Spline`)) (`self.SectionLenght`))) 1))
          (set `self.LoopIndex` _index_3)
          (for _index_4 (range 1 (`self.Height`))
            (set `self.IndexHeightCurrent` _index_4)
            (bind _returnvalue_11 (`AddComponent|NODE_AddSplineMeshComponent-9`))
            (bind _output_get_3 (set `self.SplineMeshComponent` _returnvalue_11))
            (`self.Set Spline Mesh`)
            (`StaticMeshComponent.SetStaticMesh` _output_get_3 (`self.Pillar Mesh`))
            (`SplineMeshComponent.SetForwardAxis` _returnvalue_11 "X" true)
            (bind _position (`self.Get End Pos/Tangent` _loopindex_2))
            (`SceneComponent.K2_SetRelativeTransform` (`self.SplineMeshComponent`) (`KismetMathLibrary.MakeTransform` (`KismetMathLibrary.MakeVector` (.x _position) (.y _position) (* (`self.IndexHeightCurrent`) (.z (`.Max` (`StaticMeshComponent.GetLocalBounds` (`self.SplineMeshComponent`)))) 0.0)) (`SplineComponent.GetRotationAtDistanceAlongSpline` (`self.Spline`) (* (+ _loopindex_2 1) (`self.SectionLenght`)) "Local")) false false)))))
    (:`then_2`
      ;[1 1 1] Roof Wall
      (for _index_5 (range -1 (+ (`KismetMathLibrary.FTrunc` (/ (`SplineComponent.GetSplineLength` (`self.Spline`)) (`self.SectionLenght`))) 1))
        (set `self.LoopIndex` _index_5)
        (for _index_6 (range (* _height 3) (+ (- _height (* _height -2)) 1))
          (bind _returnvalue_12 (`AddComponent|NODE_AddSplineMeshComponent-5` :`RelativeTransform` (`KismetMathLibrary.MakeTransform` (`KismetMathLibrary.MakeVector` 0.0 0.0 (* _index_6 (.z (`.Max` (`StaticMeshComponent.GetLocalBounds` (`self.SplineMeshComponent`)))))))))
          (bind _output_get_4 (set `self.SplineMeshComponent` _returnvalue_12))
          (`StaticMeshComponent.SetStaticMesh` _output_get_4 (`self.Roof End`))
          (`SplineMeshComponent.SetForwardAxis` (`self.SplineMeshComponent`) "X" true)
          (bind (_start_location _start_tangent) (`self.Get Start Pos/Tangent` (`self.LoopIndex`)))
          (bind (_position_2 _tangent) (`self.Get End Pos/Tangent` (`self.LoopIndex`)))
          (`SplineMeshComponent.SetStartAndEnd` (`self.SplineMeshComponent`) _start_location _start_tangent _position_2 _tangent false))))
    (:`then_3`
      ;[1 1 1] Wall
      (for _index_7 (range (+ (`KismetMathLibrary.FTrunc` (/ (`SplineComponent.GetSplineLength` (`self.Spline`)) (`self.SectionLenght`))) 1))
        (set `self.LoopIndex` _index_7)
        (for _index_8 (range (`self.Height`))
          (bind _output_get_5 (set `self.IndexHeightCurrent` _index_8))
          (set `self.Max Z` (.z _max))
          (bind _returnvalue_13 (`AddComponent|NODE_AddSplineMeshComponent-0` :`RelativeTransform` (`KismetMathLibrary.MakeTransform` (`KismetMathLibrary.MakeVector` 0.0 0.0 (* _output_get_5 (.z _max))))))
          (bind _output_get_6 (set `self.SplineMeshComponent` _returnvalue_13))
          (`self.Set Spline Mesh`)
          (`StaticMeshComponent.SetStaticMesh` _output_get_6 (`self.SplineMesh`))
          (`SplineMeshComponent.SetForwardAxis` (`self.SplineMeshComponent`) "X" true)
          (bind (_start_location_2 _start_tangent_2) (`self.Get Start Pos/Tangent` (`self.LoopIndex`)))
          (bind (_position_3 _tangent_2) (`self.Get End Pos/Tangent` (`self.LoopIndex`)))
          (`SplineMeshComponent.SetStartAndEnd` (`self.SplineMeshComponent`) _start_location_2 _start_tangent_2 _position_3 _tangent_2 false)
          (`KismetSystemLibrary.SphereTraceSingleByProfile` :`Radius` 55.0 :`DrawDebugType` "ForDuration"))))
    (:`then_4`
      ;[1 1 1] Floor
      (`|ExecutionSequence`
        (:`then_0`
          (if (`self.Floor Create?`)
            (for _index_9 (range (+ _returnvalue_8 1))
              (bind _returnvalue_location_4 (`KismetMathLibrary.BreakTransform` (`SplineComponent.GetTransformAtDistanceAlongSpline` _spline_2 (* (/ (`KismetMathLibrary.Conv_IntToDouble` _index_9) _returnvalue_8) _returnvalue_4) "Local" false)))
              (bind _output_get_7 (set `self.Vectors_A` (+ _returnvalue_location_4 (`self.Vectors_A`)))))
            (`KismetArrayLibrary.Array_Set` (`self.Vertices`) 0 (/ _output_get_7 _returnvalue_4))
            (for _index_10 (range (+ (`KismetMathLibrary.FTrunc` (/ (`SplineComponent.GetSplineLength` (`self.Spline`)) (`self.SectionLenght`))) 1))
              (set `self.Index B` _index_10)
              (`KismetArrayLibrary.Array_Set` _vertices 1 _returnvalue_location)
              (`KismetArrayLibrary.Array_Set` _vertices 2 _returnvalue_location_2)
              (`|ExecutionSequence`
                (:`then_0`
                  (set `self.UVs` (`|MakeArray` (0.0 0.0) (1.0 0.0) (0.0 1.0) :!type "Vector2D Structure")))
                (:`then_1`
                  (`/Engine/EditorBlueprintResources/StandardMacros.DoOnce` false
                    (:`Completed`
                      (bind (_vectices _triangles _normals _uvs _tangents) (`self.Get Section`))))))
              (`ProceduralMeshComponent.CreateMeshSection_LinearColor` :`self` (`self.ProceduralMeshFloor`) :`SectionIndex` (`self.Index B`) :`Vertices` (`self.Vertices`) :`Triangles` _triangles :`Normals` _normals :`UV0` (`self.UVs`) :`Tangents` _tangents)
              (`PrimitiveComponent.SetMaterial` (`self.ProceduralMeshFloor`) (`self.Index B`) (`self.Material Floor`)))))))
    (:`then_5`
      ;[1 1 1] Roof
      (`|ExecutionSequence`
        (:`then_0`
          (if (`self.Roof Create?`)
            (for _index_11 (range (+ _returnvalue_5 1))
              (bind _returnvalue_location_5 (`KismetMathLibrary.BreakTransform` (`SplineComponent.GetTransformAtDistanceAlongSpline` _spline_5 (* (/ (`KismetMathLibrary.Conv_IntToDouble` _index_11) _returnvalue_5) _returnvalue) "Local" false)))
              (bind _output_get_8 (set `self.Vectors` (+ _returnvalue_location_5 (`self.Vectors`)))))
            (for _ (range (`self.Height`))
              _)
            (bind (_returnvalue_x_3 _returnvalue_y_2) (`KismetMathLibrary.BreakVector` (/ _output_get_8 _returnvalue)))
            (`KismetArrayLibrary.Array_Set` (`self.Vertices`) 0 (`KismetMathLibrary.MakeVector` _returnvalue_x_3 _returnvalue_y_2 (* (`self.Height`) (.z (`.Max` (`StaticMeshComponent.GetLocalBounds` (`self.SplineMeshComponent`)))))))
            (for _index_12 (range (+ (`KismetMathLibrary.FTrunc` (/ (`SplineComponent.GetSplineLength` (`self.Spline`)) (`self.SectionLenght`))) 1))
              (set `self.Index_A` _index_12)
              (`KismetArrayLibrary.Array_Set` _vertices_2 1 (`KismetMathLibrary.MakeVector` (.x (.location _returnvalue_2)) (.y (.location _returnvalue_2)) _returnvalue_9))
              (`KismetArrayLibrary.Array_Set` _vertices_2 2 (`KismetMathLibrary.MakeVector` (.x (.location _returnvalue_6)) (.y (.location _returnvalue_6)) _returnvalue_9))
              (`|ExecutionSequence`
                (:`then_0`
                  _)
                (:`then_1`
                  (`/Engine/EditorBlueprintResources/StandardMacros.DoOnce` false
                    (:`Completed`
                      (bind (_vectices_2 _triangles_2 _normals_2) (`self.Get Section`))))))
              (`ProceduralMeshComponent.CreateMeshSection_LinearColor` :`self` (`self.ProceduralMeshRoof`) :`SectionIndex` (`self.Index_A`) :`Vertices` (`self.Vertices`) :`Triangles` _triangles_2 :`Normals` _normals_2 :`UV0` (`self.UVs`))
              (`PrimitiveComponent.SetMaterial` (`self.ProceduralMeshRoof`) (`self.Index_A`) (`self.Material Roof`)))))))
    (:`then_6`
      ;[1 1 1] Props
      (if (`self.Create Props?`)
        (for _index_13 (range (+ (`KismetMathLibrary.FTrunc` (/ (`SplineComponent.GetSplineLength` (`self.Spline`)) (`self.SectionLenght`))) 1))
          (set `self.LoopIndex` _index_13)
          (for _index_14 (range 1 (`self.Height`))
            (bind _output_get_9 (set `self.IndexHeightCurrent` _index_14))
            (bind _returnvalue_14 (`AddComponent|NODE_AddSplineMeshComponent-4` :`RelativeTransform` (`KismetMathLibrary.MakeTransform` (`KismetMathLibrary.MakeVector` 0.0 0.0 (* (.z (`.Max` (`StaticMeshComponent.GetLocalBounds` (`self.SplineMeshComponent`)))) _output_get_9)))))
            (bind _output_get_10 (set `self.SplineMeshComponent` _returnvalue_14))
            (`self.Set Spline Mesh`)
            (`StaticMeshComponent.SetStaticMesh` _output_get_10 (`self.Spline Mesh Props`))
            (`SplineMeshComponent.SetForwardAxis` (`self.SplineMeshComponent`) "X" true)
            (bind _position_4 (`self.Get End Pos/Tangent` _loopindex_3))
            (`SceneComponent.K2_SetRelativeTransform` (`self.SplineMeshComponent`) (`KismetMathLibrary.MakeTransform` (`KismetMathLibrary.MakeVector` (.x _position_4) (.y _position_4) (* (`self.Max Z`) (`self.IndexHeightCurrent`))) (`SplineComponent.GetRotationAtDistanceAlongSpline` (`self.Spline`) (* (+ _loopindex_3 1) (`self.SectionLenght`)) "Local")) false false)))))))